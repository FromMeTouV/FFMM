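; Dialogue component that runs data-table-driven conversations with a named speaker and selectable replies.
; Each interact shows the current row's text and stores its next row, table and end flag, closing the widget once the end flag is set.
; Opening creates WB_Dialogue, shows the cursor, and adds WB_Options buttons only if that first row is open-ended.
; Selecting an option clears the choices and jumps to its target row.
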(event Custom|Option%20selected
  (params (RowName :type Name) (DataTable :type Data%20Table%20Object%20Reference))
  (bind _dialoguewidget (Variables|Default|GetDialoguewidget))
  (bind _returnvalue (Utilities|GetDataTableRow DataTable RowName)
    (:then
      (Widget|Panel|ClearChildren (Variables|/Game/Interfaces/UserInterface/WB_Dialogue.WB_Dialogue_C|GetOptionscrollbox _dialoguewidget))
      (Default|UpdateDialogue _dialoguewidget (.Dialogue (Utilities|Struct|BreakDialogue_Structure _returnvalue)))
      (Variables|Default|SetRow%20Name (.Row (Utilities|Struct|BreakDialogue_Structure _returnvalue)))
      (Variables|Default|SetData%20Table (.Datatable (Utilities|Struct|BreakDialogue_Structure _returnvalue)))
      (Variables|Default|SetEnddialogue (.EndDialogue (Utilities|Struct|BreakDialogue_Structure _returnvalue))))))

(event EventBeginPlay)

(event EventTick
  (params (DeltaSeconds :type Float%20%28single-precision%29)))

(event EventInteact
  (params (playerref :type BP%20First%20Person%20Character%20Object%20Reference))
  (bind _returnvalue (Game|GetPlayerController 0))
  (bind _returnvalue_2 (Game|GetPlayerController 0))
  (if (Variables|Default|GetEnddialogue)
    (Widget|RemovefromParent (Variables|Default|GetDialoguewidget))
    (Variables|Default|SetEnddialogue false)
    (Variables|Default|SetDialoguewidget 0)
    (Input|SetInputModeGameOnly _returnvalue_2 false)
    (Variables|/Script/Engine.PlayerController|SetbShowMouseCursor _returnvalue_2 false)
    (else
      (Utilities|IsValid (Variables|Default|GetDialoguewidget)
        (:Is%20Valid
          (bind _returnvalue_3 (Utilities|GetDataTableRow (Variables|Default|GetData%20Table) (Variables|Default|GetRow%20Name))
            (:then
              (Default|UpdateDialogue (Variables|Default|GetDialoguewidget) (.Dialogue (Utilities|Struct|BreakDialogue_Structure _returnvalue_3)))
              (Variables|Default|SetRow%20Name (.Row (Utilities|Struct|BreakDialogue_Structure _returnvalue_3)))
              (Variables|Default|SetData%20Table (.Datatable (Utilities|Struct|BreakDialogue_Structure _returnvalue_3)))
              (Variables|Default|SetEnddialogue (.EndDialogue (Utilities|Struct|BreakDialogue_Structure _returnvalue_3))))))
        (:Is%20Not%20Valid
          (bind _returnvalue_4 (Utilities|GetDataTableRow (Variables|Default|GetData%20Table) (Variables|Default|GetRow%20Name))
            (:then
              (bind _returnvalue_5 (UserInterface|CreateWidget "/Game/Interfaces/UserInterface/WB_Dialogue.WB_Dialogue_C" 0 (Utilities|Text|ToText(Name) (Variables|Default|GetName)) (.Dialogue (Utilities|Struct|BreakDialogue_Structure _returnvalue_4))))
              (bind _output_get (Variables|Default|SetDialoguewidget _returnvalue_5))
              (UserInterface|Viewport|AddtoViewport _output_get 0)
              (Variables|Default|SetRow%20Name (.Row (Utilities|Struct|BreakDialogue_Structure _returnvalue_4)))
              (Variables|Default|SetData%20Table (.Datatable (Utilities|Struct|BreakDialogue_Structure _returnvalue_4)))
              (Variables|Default|SetEnddialogue (.EndDialogue (Utilities|Struct|BreakDialogue_Structure _returnvalue_4)))
              (Input|SetInputModeGameandUI _returnvalue 0 "DoNotLock" true false)
              (Variables|/Script/Engine.PlayerController|SetbShowMouseCursor _returnvalue true)
              (if (.OpenEndedDialogue? (Utilities|Struct|BreakDialogue_Structure _returnvalue_4))
                (for _array_element (.OpenEndedDialogueOptions (Utilities|Struct|BreakDialogue_Structure _returnvalue_4))
                  (bind _returnvalue_6 (UserInterface|CreateWidget "/Game/Interfaces/UserInterface/WB_Options.WB_Options_C" 0 (Utilities|Text|ToText(Name) (.Optionname (Utilities|Struct|BreakOptionsdialogue_Structure _array_element))) self (.Row (Utilities|Struct|BreakOptionsdialogue_Structure _array_element)) (.Datatable (Utilities|Struct|BreakOptionsdialogue_Structure _array_element))))
                  (Widget|Panel|AddChild (Variables|/Game/Interfaces/UserInterface/WB_Dialogue.WB_Dialogue_C|GetOptionscrollbox (Variables|Default|GetDialoguewidget)) _returnvalue_6))))))))))

(event EventLeaveDialogue
  (bind _returnvalue (Game|GetPlayerController 0))
  (Utilities|IsValid (Variables|Default|GetDialoguewidget)
    (:Is%20Valid
      (Widget|RemovefromParent (Variables|Default|GetDialoguewidget))
      (Variables|Default|SetEnddialogue false)
      (Variables|Default|SetDialoguewidget 0)
      (Input|SetInputModeGameOnly _returnvalue false)
      (Variables|/Script/Engine.PlayerController|SetbShowMouseCursor _returnvalue false))))