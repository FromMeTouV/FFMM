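; BP_Item is a pickup item that shows an interaction prompt while the player character is inside its Trigger.
; BeginPlay creates the P_Interact widget and plays a timeline that drives the static mesh's relative location.
; Trigger overlaps add the widget to the viewport and remove it.
; Interact prints a pickup message, starts a briefly delayed self-destruction and returns the item's static mesh to the caller.
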(event OnComponentBeginOverlap(Trigger)
  (params (OverlappedComponent :type Primitive%20Component%20Object%20Reference) (OtherActor :type Actor%20Object%20Reference) (OtherComp :type Primitive%20Component%20Object%20Reference) (OtherBodyIndex :type Integer) (bFromSweep :type Boolean) (SweepResult :type Hit%20Result%20Structure%20%28by%20ref%29))
  (if (== OtherActor (Game|GetPlayerCharacter 0))
    (UserInterface|Viewport|AddtoViewport (Variables|Default|GetInteractWidget) 0)))

(event OnComponentEndOverlap(Trigger)
  (params (OverlappedComponent :type Primitive%20Component%20Object%20Reference) (OtherActor :type Actor%20Object%20Reference) (OtherComp :type Primitive%20Component%20Object%20Reference) (OtherBodyIndex :type Integer))
  (if (== (Game|GetPlayerCharacter 0) OtherActor)
    (Widget|RemovefromParent (Variables|Default|GetInteractWidget))))

(event Custom|DestroyItem
  (Utilities|FlowControl|Delay 0.2)
  (Actor|DestroyActor))

(event EventBeginPlay
  (bind _returnvalue (UserInterface|CreateWidget "/Game/Blueprint/P_Interact.P_Interact_C"))
  (Variables|Default|SetInteractWidget _returnvalue)
  (bind _float_timeline (Timeline|Timeline Play)
    (:Update
      (Transformation|SetRelativeLocation (Variables|Default|GetStaticMesh) _float_timeline false false))))

(fn ConstructionScript)

(fn Interact
  (Development|PrintString "Picked Up" false)
  (CallFunction|DestroyItem)
  (return (Variables|/Script/Engine.StaticMeshComponent|GetStaticMesh (Variables|Default|GetStaticMesh))))